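; LetterPuzzleButtonBP is a clickable cube button for a letter puzzle that shows a single letter on a text component.
; On BeginPlay it writes its TheLetter variable onto the text.
; Clicking the cube converts the displayed text to a string and reports it to its TheConsole reference through AButtonIsPressed.
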(event `self.Cube.OnClicked`
  (params (TouchedComponent :type "PrimitiveComponent Object Reference"))
  (`/Game/LetterPuzzle/LetterPuzzleConsoleBP.AButtonIsPressed` (`self.TheConsole`) (`KismetTextLibrary.Conv_TextToString` (`TextRenderComponent.Text` (`self.Text`)))))

(event `self.ReceiveActorBeginOverlap`
  (params (OtherActor :type "Actor Object Reference")))

(event `self.ReceiveTick`
  (params (DeltaSeconds :type "Float (single-precision)")))

(event `self.ReceiveBeginPlay`
  (`self.SetTheLetter`))

(fn `SetTheLetter`
  (`TextRenderComponent.K2_SetText` (`self.Text`) (`KismetTextLibrary.Conv_StringToText` (`self.theLetter`)))
  (return))

(fn `UserConstructionScript`)