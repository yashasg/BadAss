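; Actor for a letter puzzle that displays a single solution letter on a cube with switchable highlighting.
; On BeginPlay, SetTheLetter copies the TheLetter variable into the Text component.
; ChangeToRed and ChangeToBlue swap the Cube's material between BaseMaterial and GlowyMat.
; Nothing in this Blueprint calls the color functions, and its overlap and tick events are empty.
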(event `self.ReceiveActorBeginOverlap`
  (params (OtherActor :type "Actor Object Reference")))

(event `self.ReceiveTick`
  (params (DeltaSeconds :type "Float (single-precision)")))

(event `/Game/LetterPuzzle/LetterPuzzleButtonBP.ReceiveBeginPlay`
  (`self.SetTheLetter`))

(fn `ChangeToBlue`
  (`PrimitiveComponent.SetMaterial` (`self.Cube`) 0 "/Game/New_Stuff/GlowyMat.GlowyMat"))

(fn `ChangeToRed`
  (`PrimitiveComponent.SetMaterial` (`self.Cube`) 0 "/Game/FirstPerson/Meshes/BaseMaterial.BaseMaterial"))

(fn `SetTheLetter`
  (`TextRenderComponent.K2_SetText` (`self.Text`) (`KismetTextLibrary.Conv_StringToText` (`self.theLetter`)))
  (return))

(fn `UserConstructionScript`)