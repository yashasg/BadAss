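; PlantPuzzleButtonBP is a button actor in the plant fan puzzle that forwards clicks to its console.
; When clicked, it calls ClickButtonAt on the referenced console with its own index, leaving the puzzle logic to that console.
; ApplyOnMat and ApplyOffMat swap the static mesh's first material to show on and off states.
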(event `self.ReceiveBeginPlay`)

(event `self.ReceiveActorBeginOverlap`
  (params (OtherActor :type "Actor Object Reference")))

(event `self.ReceiveTick`
  (params (DeltaSeconds :type "Float (single-precision)")))

(fn `ApplyOffMat`
  (`PrimitiveComponent.SetMaterial` (`self.StaticMesh`) 0 (`self.m_offMat`)))

(fn `ApplyOnMat`
  (`PrimitiveComponent.SetMaterial` (`self.StaticMesh`) 0 (`self.m_onMat`)))

(fn `PpbOnClicked`
  (`PlantPuzzleConsole.ClickButtonAt` (`self.m_console`) (`self.m_index`)))

(fn `UserConstructionScript`)